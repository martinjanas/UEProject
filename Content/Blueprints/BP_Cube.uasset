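; BP_Cube is an actor that spins and bounces while periodically draining Wood and Stone stacks in the item registry.
; Tick lerps yaw toward a 90-degree offset, scaled by RotationSpeed and delta time, and drives the Bounce component with fixed values, leaving BounceSpeed unused.
; A Delay on Tick throttles DecreaseItemsStack to roughly once per second, where it looks up both items by name and reduces their stacks.
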(event `self.ReceiveBeginPlay`
  (set `self.Rotation Speed` 1.5)
  (set `self.Bounce Speed` 1.5))

(event `self.ReceiveActorBeginOverlap`
  (params (OtherActor :type "Actor Object Reference")))

(event `self.ReceiveTick`
  (params (DeltaSeconds :type "Float (single-precision)"))
  (`self.Rotate Cube` DeltaSeconds)
  (`BounceComponent.BounceActor` (`self.Bounce`) DeltaSeconds 2.0 2.0)
  (`KismetSystemLibrary.Delay` 1.0)
  (`self.DecreaseItemsStack`))

(fn `DecreaseItemsStack`
  (bind _returnvalue (`ItemRegistry.GetItemRegistry`))
  (bind _returnvalue_2 (`ItemRegistry.FindItem` _returnvalue "Wood"))
  (`Item.RemoveStackAmount` _returnvalue_2 2)
  (bind _returnvalue_3 (`ItemRegistry.FindItem` _returnvalue "Stone"))
  (`Item.RemoveStackAmount` _returnvalue_3 1))

(fn `Rotate Cube`
  (params (`Delta Time` :type "Float (double-precision)"))
  (locals (`Rotation Speed * deltaTime` :type "Float (double-precision)"))
  (bind (_returnvalue_roll _returnvalue_pitch _returnvalue_yaw) (`KismetMathLibrary.BreakRotator` (`self.K2_GetActorRotation`)))
  (bind _output_get (set `local.Rotation Speed * deltaTime` (* `Delta Time` (`self.Rotation Speed`))))
  (`self.K2_SetActorRotation` (`KismetMathLibrary.RLerp` (`KismetMathLibrary.MakeRotator` _returnvalue_roll _returnvalue_pitch _returnvalue_yaw) (`KismetMathLibrary.MakeRotator` 0.0 0.0 (+ _returnvalue_yaw 90.0)) _output_get)))

(fn `UserConstructionScript`)